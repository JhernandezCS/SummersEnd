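; Main game player controller that starts dialogue scenes and lets the player advance through them.
; On BeginPlay it caches GM_MainGame and binds to its main HUD's text-finished event.
; StartDialogue locks progression and passes scene data to the HUD; the OK input advances only after text finishes, then locks again.
; SetCutsceneControls adds or removes the dialogue Enhanced Input mapping context to toggle cutscene controls.
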(event Custom|On%20Dialogue%20Text%20Finished
  (Variables|Default|SetCan%20Progress%20Dialog true))

(event Input|EnhancedActionEvents|EnhancedInputActionIA_Dialogue_OK
  (params (ActionValue :type Boolean) (ElapsedSeconds :type Float%20%28double-precision%29) (TriggeredSeconds :type Float%20%28double-precision%29) (InputAction :type Input%20Action%20Object%20Reference :default "/Game/Dynamic/Blueprints/Input/Actions/IA_Dialogue_OK.IA_Dialogue_OK"))
  (if (and (Variables|Default|GetCan%20Progress%20Dialog) ActionValue)
    (Default|ShowNextDialogue (Variables|/Game/Dynamic/Blueprints/Game_Modes/GM_MainGame.GM_MainGame_C|GetWBP_MainHUD (Variables|Default|GetGM_MainGame)))
    (Variables|Default|SetCan%20Progress%20Dialog false)))

(event EventBeginPlay
  (bind _asgm_main_game (Utilities|Casting|CastToGM_MainGame (Game|GetGameMode))
    (:then
      (bind _output_get (Variables|Default|SetGM_MainGame _asgm_main_game))
      (EventDispatchers|BindEventtoDialogueTextFinished (Variables|/Game/Dynamic/Blueprints/Game_Modes/GM_MainGame.GM_MainGame_C|GetWBP_MainHUD _output_get) (delegate Custom|On%20Dialogue%20Text%20Finished)))
    (:CastFailed
      (Development|PrintString "BP_MainGameController::BeingPlay failed to cast game mode to GM_MainGame"))))

(event Collision|EventActorBeginOverlap
  (params (OtherActor :type Actor%20Object%20Reference)))

(event EventTick
  (params (DeltaSeconds :type Float%20%28single-precision%29)))

(fn ConstructionScript)

(fn StartDialogue
  (params (Dialogue%20Scene%20Data :type S%20Dialogue%20Scene%20Data%20Structure))
  (Utilities|FlowControl|Sequence
    (:then_0
      (Variables|Default|SetCan%20Progress%20Dialog false))
    (:then_1
      (Default|StartDialogue (Variables|/Game/Dynamic/Blueprints/Game_Modes/GM_MainGame.GM_MainGame_C|GetWBP_MainHUD (Variables|Default|GetGM_MainGame)) Dialogue%20Scene%20Data))))

(fn SetCutsceneControls
  (params (Is%20Cutscene%20Controls :type Boolean))
  (bind _self self)
  (bind _returnvalue (PlayerController|LocalPlayerSubsystems|GetEnhancedInputLocalPlayerSubsystem _self))
  (if Is%20Cutscene%20Controls
    (Input|AddMappingContext _returnvalue "/Game/Dynamic/Blueprints/Input/IMC_Dialogue.IMC_Dialogue" 1 "(bIgnoreAllPressedKeysUntilRelease=True,bForceImmediately=False,bNotifyUserSettings=False)")
    (else
      (Input|RemoveMappingContext _returnvalue "/Game/Dynamic/Blueprints/Input/IMC_Dialogue.IMC_Dialogue" "(bIgnoreAllPressedKeysUntilRelease=True,bForceImmediately=False,bNotifyUserSettings=False)"))))