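; Cutscene manager component that coordinates the active level sequence with dialogue and screen effects.
; StartCutscene switches the player controller to cutscene controls and binds UnpauseSequence to the main HUD's scene-finished event.
; RunDialogue passes DT_Dialogue rows to the controller, while PlayEffect drives the HUD effect display and can bind its completion to UnpauseSequence.
; UnpauseSequence resumes the game mode's active sequence and removes any effect binding.
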(event Custom|Unpause%20Sequence
  (Utilities|FlowControl|Sequence
    (:then_0
      (bind _sequence_player (CallFunction|GetActiveSequence))
      (Sequencer|Player|Play _sequence_player :!class /Script/MovieScene.MovieSceneSequencePlayer))
    (:then_1
      (if (Variables|Default|GetIs%20Waiting%20For%20Effect)
        (CallFunction|BindtoEffectFinished false)))))

(event Custom|Bind%20To%20Scene%20Finished
  (params (Set%20Binding :type Boolean))
  (bind _game_mode (Variables|Default|GetGame%20Mode))
  (bind _wbp_mainhud (Variables|/Game/Dynamic/Blueprints/Game_Modes/GM_MainGame.GM_MainGame_C|GetWBP_MainHUD _game_mode))
  (if Set%20Binding
    (EventDispatchers|BindEventtoSceneFinished _wbp_mainhud (delegate Custom|Unpause%20Sequence))
    (else
      (EventDispatchers|UnbindEventfromSceneFinished _wbp_mainhud (delegate Custom|Unpause%20Sequence)))))

(event Custom|Bind%20To%20Effect%20Finished
  (params (Set%20Binding :type Boolean))
  (bind _game_mode (Variables|Default|GetGame%20Mode))
  (bind _wbp_mainhud (Variables|/Game/Dynamic/Blueprints/Game_Modes/GM_MainGame.GM_MainGame_C|GetWBP_MainHUD _game_mode))
  (bind _wbp_effectdisplay (Variables|/Game/Dynamic/Widgets/WBP_MainHUD.WBP_MainHUD_C|GetWBP_EffectDisplay _wbp_mainhud))
  (if Set%20Binding
    (EventDispatchers|BindEventtoEffectComplete _wbp_effectdisplay (delegate Custom|Unpause%20Sequence))
    (else
      (EventDispatchers|UnbindEventfromEffectComplete _wbp_effectdisplay (delegate Custom|Unpause%20Sequence)))))

(event EventBeginPlay
  (bind _asgm_main_game (Utilities|Casting|CastToGM_MainGame (Game|GetGameMode))
    (:then
      (Variables|Default|SetGame%20Mode _asgm_main_game))
    (:CastFailed
      (Development|PrintString "BPC_CustceneManager::BeginPlay Failed to cast game mode to GM_MainGame"))))

(event EventTick
  (params (DeltaSeconds :type Float%20%28single-precision%29)))

(fn StartCutscene
  (bind _asbp_main_game_controller (Utilities|Casting|CastToBP_MainGameController (Game|GetPlayerController 0)))
  (Default|SetCutsceneControls _asbp_main_game_controller true)
  (CallFunction|BindtoSceneFinished true))

(fn RunDialogue
  (params (Dialogue%20DataTable%20Name :type Name))
  (bind _asbp_main_game_controller (Utilities|Casting|CastToBP_MainGameController (Game|GetPlayerController 0)))
  (bind _returnvalue (Utilities|GetDataTableRow "/Game/Dynamic/Data_Tables/DT_Dialogue.DT_Dialogue" Dialogue%20DataTable%20Name)
    (:then
      (Default|StartDialogue _asbp_main_game_controller (Utilities|Struct|BreakS_DialogueScenes _returnvalue)))))

(fn GetActiveSequence
  (bind _asbp_main_game_controller (Utilities|Casting|CastToBP_MainGameController (Game|GetPlayerController 0))
    (:then
      (bind _asgm_main_game (Utilities|Casting|CastToGM_MainGame (Game|GetGameMode)))
      (bind _active_sequence (Default|GetActiveSequence _asgm_main_game))
      (return _active_sequence _asbp_main_game_controller))
    (:CastFailed
      (Development|PrintString "BPC_CutsceneManager::GetActiveSequence failed to cast player controller"))))

(fn PlayEffect
  (params (Effect :type ENUM_ScreenEffects%20Enum :default "NewEnumerator0") (Effect%20Image :type Texture%202D%20Object%20Reference) (Wait%20For%20Effect :type Boolean))
  (Utilities|FlowControl|Sequence
    (:then_0
      (Default|PlayEffect (Variables|/Game/Dynamic/Widgets/WBP_MainHUD.WBP_MainHUD_C|GetWBP_EffectDisplay (Variables|/Game/Dynamic/Blueprints/Game_Modes/GM_MainGame.GM_MainGame_C|GetWBP_MainHUD (Variables|Default|GetGame%20Mode))) Effect Effect%20Image))
    (:then_1
      (if Wait%20For%20Effect
        (CallFunction|BindtoEffectFinished true)
        (Variables|Default|SetIs%20Waiting%20For%20Effect true)))))