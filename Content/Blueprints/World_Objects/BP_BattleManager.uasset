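; BP_BattleManager sets up the player side of a battle and drives cursor selection on its platform grid.
; On BeginPlay it spawns each party character's battler on a shuffled platform, tints that platform to the character's color, and selects cell (0,0).
; It binds BP_BattleController's four direction events to step the selected cell through the IntPoint-keyed platform map, printing an error for invalid cells.
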(event Custom|Up%20Pressed
  (CallFunction|OnInputReceived "NewEnumerator0"))

(event Custom|Down%20Pressed
  (CallFunction|OnInputReceived "NewEnumerator1"))

(event Custom|Right%20Pressed
  (CallFunction|OnInputReceived "NewEnumerator3"))

(event Custom|Left%20Pressed
  (CallFunction|OnInputReceived "NewEnumerator2"))

(event EventBeginPlay
  (Utilities|FlowControl|Sequence
    (:then_0
      (CallFunction|SpawnPlayerSide)
      (CallFunction|SelectPlayerPlatformbyGridCell (Utilities|Struct|MakeIntPoint 0 0)))
    (:then_1
      (bind _asbp_battle_controller (Utilities|Casting|CastToBP_BattleController (Game|GetPlayerController 0)))
      (EventDispatchers|BindEventtoUpDirection _asbp_battle_controller (delegate Custom|Up%20Pressed))
      (EventDispatchers|BindEventtoDownDirection _asbp_battle_controller (delegate Custom|Down%20Pressed))
      (EventDispatchers|BindEventtoLeftDirection _asbp_battle_controller (delegate Custom|Left%20Pressed))
      (EventDispatchers|BindEventtoRightDirection _asbp_battle_controller (delegate Custom|Right%20Pressed)))))

(event Collision|EventActorBeginOverlap
  (params (OtherActor :type Actor%20Object%20Reference)))

(event EventTick
  (params (DeltaSeconds :type Float%20%28single-precision%29)))

(fn ConstructionScript)

(fn BattleCharactertoClass
  (params (Character :type ENUM_BattleCharacters%20Enum :default "NewEnumerator0"))
  (switch Utilities|FlowControl|Switch|SwitchonENUM_BattleCharacters Character
    (:NewEnumerator0
      (return "/Game/Blueprints/Characters/BB/BattleMode/BP_BB_Battler.BP_BB_Battler_C"))
    (:NewEnumerator1
      (return "/Game/Blueprints/Characters/Daisy/BattleMode/BP_Daisy_Battler.BP_Daisy_Battler_C"))
    (:NewEnumerator2
      (return "/Game/Blueprints/Characters/Tori/BattleMode/BP_Tori_Battler.BP_Tori_Battler_C"))
    (:NewEnumerator3
      (return "/Game/Blueprints/Characters/Jay/BP_Jay.BP_Jay_C"))
    (:NewEnumerator4
      (return "/Game/Blueprints/Characters/Lottie/BP_Lottie.BP_Lottie_C"))
    (:NewEnumerator5
      (return "/Game/Blueprints/Characters/Shio/BP_Shio.BP_Shio_C"))))

(fn SpawnPlayerSide
  (bind _self self)
  (bind _color_platforms_player (Variables|Default|GetColor%20Platforms%20Player))
  (if (Utilities|Map|IsEmpty _color_platforms_player)
    (Development|PrintString "BP_BattleManager::OnSpawnPlayerSide the platforms member var was empty" true true "(R=1.000000,G=0.000000,B=0.007402,A=1.000000)" 1e+01)
    (else
      (bind _values (Utilities|Map|Values _color_platforms_player))
      (Utilities|Array|Shuffle _values)
      (bind (_array_element _array_index) (Utilities|Array|ForEachLoopwithBreak (Variables|Default|GetPlayer%20Characters%20in%20Battle))
        (:LoopBody
          (Utilities|FlowControl|Sequence
            (:then_0
              (switch Utilities|FlowControl|Switch|SwitchonENUM_BattleCharacters _array_element
                (:NewEnumerator0
                  (bind _returnvalue (Game|SpawnActorfromClass "/Game/Blueprints/Characters/BB/BattleMode/BP_BB_Battler.BP_BB_Battler_C" (Math|Transform|MakeTransform (Math|Vector|MakeVector (.X (Math|Vector|BreakVector (Transformation|GetWorldLocation (Variables|/Game/Blueprints/World_Objects/ColorPlatform/BP_ColorPlatform.BP_ColorPlatform_C|GetDefaultSceneRoot (Utilities|Array|Get(acopy) _values _array_index))))) (- (.Y (Math|Vector|BreakVector (Transformation|GetWorldLocation (Variables|/Game/Blueprints/World_Objects/ColorPlatform/BP_ColorPlatform.BP_ColorPlatform_C|GetDefaultSceneRoot (Utilities|Array|Get(acopy) _values _array_index))))) 25.0) (+ (.Z (Math|Vector|BreakVector (Transformation|GetWorldLocation (Variables|/Game/Blueprints/World_Objects/ColorPlatform/BP_ColorPlatform.BP_ColorPlatform_C|GetDefaultSceneRoot (Utilities|Array|Get(acopy) _values _array_index))))) 1e+01))) "AlwaysSpawn" "MultiplyWithRoot" _self 0))
                  (LocalVariables|SetCreated%20Player _returnvalue))
                (:NewEnumerator1
                  (bind _returnvalue_2 (Game|SpawnActorfromClass "/Game/Blueprints/Characters/Daisy/BattleMode/BP_Daisy_Battler.BP_Daisy_Battler_C" (Math|Transform|MakeTransform (Math|Vector|MakeVector (.X (Math|Vector|BreakVector (Transformation|GetWorldLocation (Variables|/Game/Blueprints/World_Objects/ColorPlatform/BP_ColorPlatform.BP_ColorPlatform_C|GetDefaultSceneRoot (Utilities|Array|Get(acopy) _values _array_index))))) (- (.Y (Math|Vector|BreakVector (Transformation|GetWorldLocation (Variables|/Game/Blueprints/World_Objects/ColorPlatform/BP_ColorPlatform.BP_ColorPlatform_C|GetDefaultSceneRoot (Utilities|Array|Get(acopy) _values _array_index))))) 25.0) (+ (.Z (Math|Vector|BreakVector (Transformation|GetWorldLocation (Variables|/Game/Blueprints/World_Objects/ColorPlatform/BP_ColorPlatform.BP_ColorPlatform_C|GetDefaultSceneRoot (Utilities|Array|Get(acopy) _values _array_index))))) 1e+01))) "AlwaysSpawn" "MultiplyWithRoot" _self 0))
                  (LocalVariables|SetCreated%20Player _returnvalue_2))
                (:NewEnumerator2
                  (bind _returnvalue_3 (Game|SpawnActorfromClass "/Game/Blueprints/Characters/Tori/BattleMode/BP_Tori_Battler.BP_Tori_Battler_C" (Math|Transform|MakeTransform (Math|Vector|MakeVector (.X (Math|Vector|BreakVector (Transformation|GetWorldLocation (Variables|/Game/Blueprints/World_Objects/ColorPlatform/BP_ColorPlatform.BP_ColorPlatform_C|GetDefaultSceneRoot (Utilities|Array|Get(acopy) _values _array_index))))) (- (.Y (Math|Vector|BreakVector (Transformation|GetWorldLocation (Variables|/Game/Blueprints/World_Objects/ColorPlatform/BP_ColorPlatform.BP_ColorPlatform_C|GetDefaultSceneRoot (Utilities|Array|Get(acopy) _values _array_index))))) 25.0) (+ (.Z (Math|Vector|BreakVector (Transformation|GetWorldLocation (Variables|/Game/Blueprints/World_Objects/ColorPlatform/BP_ColorPlatform.BP_ColorPlatform_C|GetDefaultSceneRoot (Utilities|Array|Get(acopy) _values _array_index))))) 1e+01))) "AlwaysSpawn" "MultiplyWithRoot" _self 0))
                  (LocalVariables|SetCreated%20Player _returnvalue_3))
                (:NewEnumerator3
                  (bind _returnvalue_4 (Game|SpawnActorfromClass "/Game/Blueprints/Characters/Jay/BattleMode/BP_Jay_Battler.BP_Jay_Battler_C" (Math|Transform|MakeTransform (Math|Vector|MakeVector (.X (Math|Vector|BreakVector (Transformation|GetWorldLocation (Variables|/Game/Blueprints/World_Objects/ColorPlatform/BP_ColorPlatform.BP_ColorPlatform_C|GetDefaultSceneRoot (Utilities|Array|Get(acopy) _values _array_index))))) (- (.Y (Math|Vector|BreakVector (Transformation|GetWorldLocation (Variables|/Game/Blueprints/World_Objects/ColorPlatform/BP_ColorPlatform.BP_ColorPlatform_C|GetDefaultSceneRoot (Utilities|Array|Get(acopy) _values _array_index))))) 25.0) (+ (.Z (Math|Vector|BreakVector (Transformation|GetWorldLocation (Variables|/Game/Blueprints/World_Objects/ColorPlatform/BP_ColorPlatform.BP_ColorPlatform_C|GetDefaultSceneRoot (Utilities|Array|Get(acopy) _values _array_index))))) 1e+01))) "AlwaysSpawn" "MultiplyWithRoot" 0 0))
                  (LocalVariables|SetCreated%20Player _returnvalue_4))
                (:NewEnumerator4
                  (bind _returnvalue_5 (Game|SpawnActorfromClass "/Game/Blueprints/Characters/Lottie/BattleMode/BP_Lottie_Battler.BP_Lottie_Battler_C" (Math|Transform|MakeTransform (Math|Vector|MakeVector (.X (Math|Vector|BreakVector (Transformation|GetWorldLocation (Variables|/Game/Blueprints/World_Objects/ColorPlatform/BP_ColorPlatform.BP_ColorPlatform_C|GetDefaultSceneRoot (Utilities|Array|Get(acopy) _values _array_index))))) (- (.Y (Math|Vector|BreakVector (Transformation|GetWorldLocation (Variables|/Game/Blueprints/World_Objects/ColorPlatform/BP_ColorPlatform.BP_ColorPlatform_C|GetDefaultSceneRoot (Utilities|Array|Get(acopy) _values _array_index))))) 25.0) (+ (.Z (Math|Vector|BreakVector (Transformation|GetWorldLocation (Variables|/Game/Blueprints/World_Objects/ColorPlatform/BP_ColorPlatform.BP_ColorPlatform_C|GetDefaultSceneRoot (Utilities|Array|Get(acopy) _values _array_index))))) 1e+01))) "AlwaysSpawn" "MultiplyWithRoot" 0 0))
                  (LocalVariables|SetCreated%20Player _returnvalue_5))
                (:NewEnumerator5
                  (bind _returnvalue_6 (Game|SpawnActorfromClass "/Game/Blueprints/Characters/Shio/BattleMode/BP_Shio_Battler.BP_Shio_Battler_C" (Math|Transform|MakeTransform (Math|Vector|MakeVector (.X (Math|Vector|BreakVector (Transformation|GetWorldLocation (Variables|/Game/Blueprints/World_Objects/ColorPlatform/BP_ColorPlatform.BP_ColorPlatform_C|GetDefaultSceneRoot (Utilities|Array|Get(acopy) _values _array_index))))) (- (.Y (Math|Vector|BreakVector (Transformation|GetWorldLocation (Variables|/Game/Blueprints/World_Objects/ColorPlatform/BP_ColorPlatform.BP_ColorPlatform_C|GetDefaultSceneRoot (Utilities|Array|Get(acopy) _values _array_index))))) 25.0) (+ (.Z (Math|Vector|BreakVector (Transformation|GetWorldLocation (Variables|/Game/Blueprints/World_Objects/ColorPlatform/BP_ColorPlatform.BP_ColorPlatform_C|GetDefaultSceneRoot (Utilities|Array|Get(acopy) _values _array_index))))) 1e+01))) "AlwaysSpawn" "MultiplyWithRoot" 0 0))
                  (LocalVariables|SetCreated%20Player _returnvalue_6))))
            (:then_1
              (Sprite|SetSpriteColor (Variables|/Game/Blueprints/World_Objects/ColorPlatform/BP_ColorPlatform.BP_ColorPlatform_C|GetPaperSprite (Utilities|Array|Get(acopy) _values _array_index)) (Default|GetCharacterColor (LocalVariables|GetCreated%20Player)))
              (Default|SetDirectionality (LocalVariables|GetCreated%20Player) "NewEnumerator0"))))))))

(fn OnInputReceived
  (params (Direction :type ENUM_BattleInputDirections%20Enum :default "ENUM_BattleInputDirections_MAX"))
  (switch Utilities|FlowControl|Switch|SwitchonENUM_BattleInputReceivers (Variables|Default|GetInput%20Mode)
    (:NewEnumerator0
      (bind _output_get (LocalVariables|SetSelected%20Cell%20Proxy (Variables|Default|GetSelected%20Cell)))
      (switch Utilities|FlowControl|Switch|SwitchonENUM_BattleInputDirections Direction
        (:NewEnumerator0
          (bind _result (Math|Integer|DecrementInt (.Y (Utilities|Struct|BreakIntPoint _output_get)))
            (:%20%20
              (CallFunction|SelectPlayerPlatformbyGridCell (Utilities|Struct|MakeIntPoint (.X (Utilities|Struct|BreakIntPoint _output_get)) _result)))))
        (:NewEnumerator1
          (bind _result_2 (Math|Integer|IncrementInt (.Y (Utilities|Struct|BreakIntPoint _output_get)))
            (:%20%20
              (CallFunction|SelectPlayerPlatformbyGridCell (Utilities|Struct|MakeIntPoint (.X (Utilities|Struct|BreakIntPoint _output_get)) _result_2)))))
        (:NewEnumerator2
          (bind _result_3 (Math|Integer|DecrementInt (.X (Utilities|Struct|BreakIntPoint _output_get)))
            (:%20%20
              (CallFunction|SelectPlayerPlatformbyGridCell (Utilities|Struct|MakeIntPoint _result_3 (.Y (Utilities|Struct|BreakIntPoint _output_get)))))))
        (:NewEnumerator3
          (bind _result_4 (Math|Integer|IncrementInt (.X (Utilities|Struct|BreakIntPoint _output_get)))
            (:%20%20
              (CallFunction|SelectPlayerPlatformbyGridCell (Utilities|Struct|MakeIntPoint _result_4 (.Y (Utilities|Struct|BreakIntPoint _output_get)))))))))))

(fn SelectPlayerPlatformbyGridCell
  (params (Index :type Int%20Point%20Structure))
  (bind _color_platforms_player (Variables|Default|GetColor%20Platforms%20Player))
  (bind (_value _returnvalue) (Utilities|Map|Find _color_platforms_player Index))
  (if (Utilities|Map|IsEmpty _color_platforms_player)
    (Development|PrintString "Select Player Platform By Index:: Player Platforms empty" true true "(R=1.000000,G=0.146882,B=0.000000,A=1.000000)" 1e+01)
    (return 0)
    (elif (not _returnvalue)
      (Development|PrintString "Select Player Platform By Index:: Invalid Cell" true true "(R=1.000000,G=0.146882,B=0.000000,A=1.000000)" 1e+01)
      (return 0)
      (else
        (Utilities|FlowControl|Sequence
          (:then_0
            (Default|SetSelected (.Value (Utilities|Map|Find _color_platforms_player (Variables|Default|GetSelected%20Cell))) false))
          (:then_1
            (Default|SetSelected _value true))
          (:then_2
            (Variables|Default|SetSelected%20Cell Index)
            (return _value)))))))