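; Battle manager actor that spawns the player's party onto color platforms when play begins.
; SpawnPlayerSide shuffles the player-side platforms, then spawns a character-specific battler slightly offset above each, tinting the platform to that character's color and setting its directionality.
; An empty platform array only prints an error.
; A separate BattleCharacterToClass lookup is unused here and returns non-Battler classes for Jay, Lottie and Shio, unlike the spawn switch.
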(event EventBeginPlay
  (CallFunction|SpawnPlayerSide))

(event Collision|EventActorBeginOverlap
  (params (OtherActor :type Actor%20Object%20Reference)))

(event EventTick
  (params (DeltaSeconds :type Float%20%28single-precision%29)))

(fn ConstructionScript)

(fn BattleCharactertoClass
  (params (Character :type ENUM_BattleCharacters%20Enum :default "NewEnumerator0"))
  (switch Utilities|FlowControl|Switch|SwitchonENUM_BattleCharacters Character
    (:NewEnumerator0
      (return "/Game/Blueprints/Characters/BB/BattleMode/BP_BB_Battler.BP_BB_Battler_C"))
    (:NewEnumerator1
      (return "/Game/Blueprints/Characters/Daisy/BattleMode/BP_Daisy_Battler.BP_Daisy_Battler_C"))
    (:NewEnumerator2
      (return "/Game/Blueprints/Characters/Tori/BattleMode/BP_Tori_Battler.BP_Tori_Battler_C"))
    (:NewEnumerator3
      (return "/Game/Blueprints/Characters/Jay/BP_Jay.BP_Jay_C"))
    (:NewEnumerator4
      (return "/Game/Blueprints/Characters/Lottie/BP_Lottie.BP_Lottie_C"))
    (:NewEnumerator5
      (return "/Game/Blueprints/Characters/Shio/BP_Shio.BP_Shio_C"))))

(fn SpawnPlayerSide
  (bind _self self)
  (bind _color_platforms_of_player_side (Variables|Default|GetColor%20Platforms%20of%20Player%20Side))
  (if (Utilities|Array|IsEmpty _color_platforms_of_player_side)
    (Development|PrintString "BP_BattleManager::OnSpawnPlayerSide the platforms member var was empty" true true "(R=1.000000,G=0.000000,B=0.007402,A=1.000000)" 1e+01)
    (else
      (Utilities|Array|Shuffle _color_platforms_of_player_side)
      (bind (_array_element _array_index) (Utilities|Array|ForEachLoopwithBreak (Variables|Default|GetPlayer%20Characters%20in%20Battle))
        (:LoopBody
          (Utilities|FlowControl|Sequence
            (:then_0
              (switch Utilities|FlowControl|Switch|SwitchonENUM_BattleCharacters _array_element
                (:NewEnumerator0
                  (bind _returnvalue (Game|SpawnActorfromClass "/Game/Blueprints/Characters/BB/BattleMode/BP_BB_Battler.BP_BB_Battler_C" (Math|Transform|MakeTransform (Math|Vector|MakeVector (.X (Math|Vector|BreakVector (Transformation|GetWorldLocation (Variables|/Game/Blueprints/World_Objects/ColorPlatform/BP_ColorPlatform.BP_ColorPlatform_C|GetDefaultSceneRoot (Utilities|Array|Get(acopy) _color_platforms_of_player_side _array_index))))) (- (.Y (Math|Vector|BreakVector (Transformation|GetWorldLocation (Variables|/Game/Blueprints/World_Objects/ColorPlatform/BP_ColorPlatform.BP_ColorPlatform_C|GetDefaultSceneRoot (Utilities|Array|Get(acopy) _color_platforms_of_player_side _array_index))))) 25.0) (+ (.Z (Math|Vector|BreakVector (Transformation|GetWorldLocation (Variables|/Game/Blueprints/World_Objects/ColorPlatform/BP_ColorPlatform.BP_ColorPlatform_C|GetDefaultSceneRoot (Utilities|Array|Get(acopy) _color_platforms_of_player_side _array_index))))) 1e+01))) "AlwaysSpawn" "MultiplyWithRoot" _self 0))
                  (LocalVariables|SetCreated%20Player _returnvalue))
                (:NewEnumerator1
                  (bind _returnvalue_2 (Game|SpawnActorfromClass "/Game/Blueprints/Characters/Daisy/BattleMode/BP_Daisy_Battler.BP_Daisy_Battler_C" (Math|Transform|MakeTransform (Math|Vector|MakeVector (.X (Math|Vector|BreakVector (Transformation|GetWorldLocation (Variables|/Game/Blueprints/World_Objects/ColorPlatform/BP_ColorPlatform.BP_ColorPlatform_C|GetDefaultSceneRoot (Utilities|Array|Get(acopy) _color_platforms_of_player_side _array_index))))) (- (.Y (Math|Vector|BreakVector (Transformation|GetWorldLocation (Variables|/Game/Blueprints/World_Objects/ColorPlatform/BP_ColorPlatform.BP_ColorPlatform_C|GetDefaultSceneRoot (Utilities|Array|Get(acopy) _color_platforms_of_player_side _array_index))))) 25.0) (+ (.Z (Math|Vector|BreakVector (Transformation|GetWorldLocation (Variables|/Game/Blueprints/World_Objects/ColorPlatform/BP_ColorPlatform.BP_ColorPlatform_C|GetDefaultSceneRoot (Utilities|Array|Get(acopy) _color_platforms_of_player_side _array_index))))) 1e+01))) "AlwaysSpawn" "MultiplyWithRoot" _self 0))
                  (LocalVariables|SetCreated%20Player _returnvalue_2))
                (:NewEnumerator2
                  (bind _returnvalue_3 (Game|SpawnActorfromClass "/Game/Blueprints/Characters/Tori/BattleMode/BP_Tori_Battler.BP_Tori_Battler_C" (Math|Transform|MakeTransform (Math|Vector|MakeVector (.X (Math|Vector|BreakVector (Transformation|GetWorldLocation (Variables|/Game/Blueprints/World_Objects/ColorPlatform/BP_ColorPlatform.BP_ColorPlatform_C|GetDefaultSceneRoot (Utilities|Array|Get(acopy) _color_platforms_of_player_side _array_index))))) (- (.Y (Math|Vector|BreakVector (Transformation|GetWorldLocation (Variables|/Game/Blueprints/World_Objects/ColorPlatform/BP_ColorPlatform.BP_ColorPlatform_C|GetDefaultSceneRoot (Utilities|Array|Get(acopy) _color_platforms_of_player_side _array_index))))) 25.0) (+ (.Z (Math|Vector|BreakVector (Transformation|GetWorldLocation (Variables|/Game/Blueprints/World_Objects/ColorPlatform/BP_ColorPlatform.BP_ColorPlatform_C|GetDefaultSceneRoot (Utilities|Array|Get(acopy) _color_platforms_of_player_side _array_index))))) 1e+01))) "AlwaysSpawn" "MultiplyWithRoot" _self 0))
                  (LocalVariables|SetCreated%20Player _returnvalue_3))
                (:NewEnumerator3
                  (bind _returnvalue_4 (Game|SpawnActorfromClass "/Game/Blueprints/Characters/Jay/BattleMode/BP_Jay_Battler.BP_Jay_Battler_C" (Math|Transform|MakeTransform (Math|Vector|MakeVector (.X (Math|Vector|BreakVector (Transformation|GetWorldLocation (Variables|/Game/Blueprints/World_Objects/ColorPlatform/BP_ColorPlatform.BP_ColorPlatform_C|GetDefaultSceneRoot (Utilities|Array|Get(acopy) _color_platforms_of_player_side _array_index))))) (- (.Y (Math|Vector|BreakVector (Transformation|GetWorldLocation (Variables|/Game/Blueprints/World_Objects/ColorPlatform/BP_ColorPlatform.BP_ColorPlatform_C|GetDefaultSceneRoot (Utilities|Array|Get(acopy) _color_platforms_of_player_side _array_index))))) 25.0) (+ (.Z (Math|Vector|BreakVector (Transformation|GetWorldLocation (Variables|/Game/Blueprints/World_Objects/ColorPlatform/BP_ColorPlatform.BP_ColorPlatform_C|GetDefaultSceneRoot (Utilities|Array|Get(acopy) _color_platforms_of_player_side _array_index))))) 1e+01))) "AlwaysSpawn" "MultiplyWithRoot" 0 0))
                  (LocalVariables|SetCreated%20Player _returnvalue_4))
                (:NewEnumerator4
                  (bind _returnvalue_5 (Game|SpawnActorfromClass "/Game/Blueprints/Characters/Lottie/BattleMode/BP_Lottie_Battler.BP_Lottie_Battler_C" (Math|Transform|MakeTransform (Math|Vector|MakeVector (.X (Math|Vector|BreakVector (Transformation|GetWorldLocation (Variables|/Game/Blueprints/World_Objects/ColorPlatform/BP_ColorPlatform.BP_ColorPlatform_C|GetDefaultSceneRoot (Utilities|Array|Get(acopy) _color_platforms_of_player_side _array_index))))) (- (.Y (Math|Vector|BreakVector (Transformation|GetWorldLocation (Variables|/Game/Blueprints/World_Objects/ColorPlatform/BP_ColorPlatform.BP_ColorPlatform_C|GetDefaultSceneRoot (Utilities|Array|Get(acopy) _color_platforms_of_player_side _array_index))))) 25.0) (+ (.Z (Math|Vector|BreakVector (Transformation|GetWorldLocation (Variables|/Game/Blueprints/World_Objects/ColorPlatform/BP_ColorPlatform.BP_ColorPlatform_C|GetDefaultSceneRoot (Utilities|Array|Get(acopy) _color_platforms_of_player_side _array_index))))) 1e+01))) "AlwaysSpawn" "MultiplyWithRoot" 0 0))
                  (LocalVariables|SetCreated%20Player _returnvalue_5))
                (:NewEnumerator5
                  (bind _returnvalue_6 (Game|SpawnActorfromClass "/Game/Blueprints/Characters/Shio/BattleMode/BP_Shio_Battler.BP_Shio_Battler_C" (Math|Transform|MakeTransform (Math|Vector|MakeVector (.X (Math|Vector|BreakVector (Transformation|GetWorldLocation (Variables|/Game/Blueprints/World_Objects/ColorPlatform/BP_ColorPlatform.BP_ColorPlatform_C|GetDefaultSceneRoot (Utilities|Array|Get(acopy) _color_platforms_of_player_side _array_index))))) (- (.Y (Math|Vector|BreakVector (Transformation|GetWorldLocation (Variables|/Game/Blueprints/World_Objects/ColorPlatform/BP_ColorPlatform.BP_ColorPlatform_C|GetDefaultSceneRoot (Utilities|Array|Get(acopy) _color_platforms_of_player_side _array_index))))) 25.0) (+ (.Z (Math|Vector|BreakVector (Transformation|GetWorldLocation (Variables|/Game/Blueprints/World_Objects/ColorPlatform/BP_ColorPlatform.BP_ColorPlatform_C|GetDefaultSceneRoot (Utilities|Array|Get(acopy) _color_platforms_of_player_side _array_index))))) 1e+01))) "AlwaysSpawn" "MultiplyWithRoot" 0 0))
                  (LocalVariables|SetCreated%20Player _returnvalue_6))))
            (:then_1
              (Sprite|SetSpriteColor (Variables|/Game/Blueprints/World_Objects/ColorPlatform/BP_ColorPlatform.BP_ColorPlatform_C|GetPaperSprite (Utilities|Array|Get(acopy) _color_platforms_of_player_side _array_index)) (Default|GetCharacterColor (LocalVariables|GetCreated%20Player)))
              (Default|SetDirectionality (LocalVariables|GetCreated%20Player) "NewEnumerator0"))))))))