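; Battle manager for the grid-based battle mode: spawns the player party on shuffled, color-tinted platforms and routes controller input.
; An input-mode state machine moves the hover cursor or forwards input to the battle HUD, stepping through platform, action, target and sub-action selection.
; Choices accumulate in nested event contexts, with actions executing once all targets are picked and undone on cancel.
; Move actions bind delegates that swap battlers between cells.
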(event Custom|Up%20Pressed
  (CallFunction|InputStateMachineTick "NewEnumerator0"))

(event Custom|Battle%20Move%20Action%20Execute%20Delegate
  (params (Context :type Battle%20Event%20Context%20Object%20Reference))
  (bind _m_sourcecell (Variables|/Script/SummersEnd.BattleEventContext|Getm_sourceCell Context))
  (bind _m_targetcells (Variables|/Script/SummersEnd.BattleEventContext|Getm_targetCells Context))
  (bind _output (Utilities|Array|Get(acopy) _m_targetcells))
  (CallFunction|SwapObjectsatCells _m_sourcecell _output)
  (CallFunction|HoverbyGridCell (Variables|/Script/SummersEnd.SBattleGridCellData|Getm_cell _output) (Variables|/Script/SummersEnd.SBattleGridCellData|Getm_cell _m_sourcecell))
  (CallFunction|GetActiveEvent)
  (CallFunction|SetInputMode "NewEnumerator6"))

(event Custom|Right%20Pressed
  (CallFunction|InputStateMachineTick "NewEnumerator3"))

(event Custom|Left%20Pressed
  (CallFunction|InputStateMachineTick "NewEnumerator2"))

(event Custom|Interact%20Executed
  (CallFunction|InputStateMachineTick "NewEnumerator4"))

(event Custom|Cancel%20Executed
  (CallFunction|InputStateMachineTick "NewEnumerator5"))

(event Custom|Bind%20To%20Battle%20Action%20Event
  (params (Action :type Battle%20Action%20Base%20Object%20Reference))
  (switch Utilities|FlowControl|Switch|SwitchonEBattleActionTypes (Class|BattleActionBase|GetBattleActionType Action)
    (:Move
      (EventDispatchers|BindEventtoOnBattleExecute Action (delegate Custom|Battle%20Move%20Action%20Execute%20Delegate))
      (EventDispatchers|BindEventtoOnBattleUndo Action (delegate Custom|Battle%20Move%20Action%20Undo%20Delegate)))))

(event Custom|Down%20Pressed
  (CallFunction|InputStateMachineTick "NewEnumerator1"))

(event Custom|Battle%20Move%20Action%20Undo%20Delegate
  (params (Context :type Battle%20Event%20Context%20Object%20Reference))
  (bind _m_sourcecell (Variables|/Script/SummersEnd.BattleEventContext|Getm_sourceCell Context))
  (bind _m_targetcells (Variables|/Script/SummersEnd.BattleEventContext|Getm_targetCells Context))
  (bind _output (Utilities|Array|Get(acopy) _m_targetcells))
  (if (Utilities|Array|IsEmpty _m_targetcells)
    (Development|PrintString "BP_BattleManagerMoveUndo:: Target cells of current context were empty. There should be at least 1.")
    (else
      (CallFunction|SwapObjectsatCells _m_sourcecell _output)
      (CallFunction|HoverbyGridCell (Variables|/Script/SummersEnd.SBattleGridCellData|Getm_cell _m_sourcecell) (Variables|/Script/SummersEnd.SBattleGridCellData|Getm_cell _output))
      (CallFunction|GetActiveEvent))))

(event EventBeginPlay
  (bind _self self)
  (Utilities|FlowControl|Sequence
    (:then_0
      (bind _asgm_battle (Utilities|Casting|CastToGM_Battle (Game|GetGameMode)))
      (bind _output_get (Variables|Default|SetBattle%20Game%20Mode _asgm_battle))
      (Default|SetBattleManager _output_get _self)
      (bind _returnvalue (Class|BattleFunctionLibraryFactory|CreateUBattleEventContext _self))
      (Utilities|Array|Add (Variables|Default|GetEvent%20Queue) _returnvalue))
    (:then_1
      (CallFunction|SpawnPlayerSide)
      (CallFunction|HoverbyGridCell (Utilities|Struct|MakeIntPoint 0 0)))
    (:then_2
      (bind _asbp_battle_controller (Utilities|Casting|CastToBP_BattleController (Game|GetPlayerController 0)))
      (EventDispatchers|BindEventtoUpDirection _asbp_battle_controller (delegate Custom|Up%20Pressed))
      (EventDispatchers|BindEventtoDownDirection _asbp_battle_controller (delegate Custom|Down%20Pressed))
      (EventDispatchers|BindEventtoLeftDirection _asbp_battle_controller (delegate Custom|Left%20Pressed))
      (EventDispatchers|BindEventtoRightDirection _asbp_battle_controller (delegate Custom|Right%20Pressed))
      (EventDispatchers|BindEventtoInteractExecuted _asbp_battle_controller (delegate Custom|Interact%20Executed))
      (EventDispatchers|BindEventtoCancelExecuted _asbp_battle_controller (delegate Custom|Cancel%20Executed)))))

(event Collision|EventActorBeginOverlap
  (params (OtherActor :type Actor%20Object%20Reference)))

(event EventTick
  (params (DeltaSeconds :type Float%20%28single-precision%29)))

(fn ConstructionScript)

(fn BattleCharactertoClass
  (params (Character :type ENUM_BattleCharacters%20Enum :default "NewEnumerator0"))
  (switch Utilities|FlowControl|Switch|SwitchonENUM_BattleCharacters Character
    (:NewEnumerator0
      (return "/Game/Blueprints/Characters/BB/BattleMode/BP_BB_Battler.BP_BB_Battler_C"))
    (:NewEnumerator1
      (return "/Game/Blueprints/Characters/Daisy/BattleMode/BP_Daisy_Battler.BP_Daisy_Battler_C"))
    (:NewEnumerator2
      (return "/Game/Blueprints/Characters/Tori/BattleMode/BP_Tori_Battler.BP_Tori_Battler_C"))
    (:NewEnumerator3
      (return "/Game/Blueprints/Characters/Jay/BP_Jay.BP_Jay_C"))
    (:NewEnumerator4
      (return "/Game/Blueprints/Characters/Lottie/BP_Lottie.BP_Lottie_C"))
    (:NewEnumerator5
      (return "/Game/Blueprints/Characters/Shio/BP_Shio.BP_Shio_C"))))

(fn SpawnPlayerSide
  (bind _self self)
  (bind _player_platforms (Variables|Default|GetPlayer%20Platforms))
  (bind _gridcells (Utilities|Struct|BreakSTRUCT_BattleGridCellCollection _player_platforms))
  (if (Utilities|Map|IsEmpty _gridcells)
    (Development|PrintString "BP_BattleManager::OnSpawnPlayerSide the platforms member var was empty" true true "(R=1.000000,G=0.000000,B=0.007402,A=1.000000)" 1e+01)
    (else
      (bind _values (Utilities|Map|Values _gridcells))
      (Utilities|Array|Shuffle _values)
      (bind (_array_element _array_index) (Utilities|Array|ForEachLoopwithBreak (Variables|Default|GetPlayer%20Characters%20in%20Battle))
        (:LoopBody
          (Utilities|FlowControl|Sequence
            (:then_0
              (switch Utilities|FlowControl|Switch|SwitchonENUM_BattleCharacters _array_element
                (:NewEnumerator0
                  (bind _returnvalue (Game|SpawnActorfromClass "/Game/Blueprints/Characters/BB/BattleMode/BP_BB_Battler.BP_BB_Battler_C" (Math|Transform|MakeTransform (Math|Vector|MakeVector (.X (Math|Vector|BreakVector (Transformation|GetWorldLocation (Variables|/Game/Blueprints/Game_Modes/BattleMode/BP_ColorPlatform.BP_ColorPlatform_C|GetDefaultSceneRoot (Utilities|Array|Get(acopy) _values _array_index))))) (- (.Y (Math|Vector|BreakVector (Transformation|GetWorldLocation (Variables|/Game/Blueprints/Game_Modes/BattleMode/BP_ColorPlatform.BP_ColorPlatform_C|GetDefaultSceneRoot (Utilities|Array|Get(acopy) _values _array_index))))) 25.0) (+ (.Z (Math|Vector|BreakVector (Transformation|GetWorldLocation (Variables|/Game/Blueprints/Game_Modes/BattleMode/BP_ColorPlatform.BP_ColorPlatform_C|GetDefaultSceneRoot (Utilities|Array|Get(acopy) _values _array_index))))) 1e+01))) "AlwaysSpawn" "MultiplyWithRoot" _self 0))
                  (LocalVariables|SetCreated%20Player _returnvalue))
                (:NewEnumerator1
                  (bind _returnvalue_2 (Game|SpawnActorfromClass "/Game/Blueprints/Characters/Daisy/BattleMode/BP_Daisy_Battler.BP_Daisy_Battler_C" (Math|Transform|MakeTransform (Math|Vector|MakeVector (.X (Math|Vector|BreakVector (Transformation|GetWorldLocation (Variables|/Game/Blueprints/Game_Modes/BattleMode/BP_ColorPlatform.BP_ColorPlatform_C|GetDefaultSceneRoot (Utilities|Array|Get(acopy) _values _array_index))))) (- (.Y (Math|Vector|BreakVector (Transformation|GetWorldLocation (Variables|/Game/Blueprints/Game_Modes/BattleMode/BP_ColorPlatform.BP_ColorPlatform_C|GetDefaultSceneRoot (Utilities|Array|Get(acopy) _values _array_index))))) 25.0) (+ (.Z (Math|Vector|BreakVector (Transformation|GetWorldLocation (Variables|/Game/Blueprints/Game_Modes/BattleMode/BP_ColorPlatform.BP_ColorPlatform_C|GetDefaultSceneRoot (Utilities|Array|Get(acopy) _values _array_index))))) 1e+01))) "AlwaysSpawn" "MultiplyWithRoot" _self 0))
                  (LocalVariables|SetCreated%20Player _returnvalue_2))
                (:NewEnumerator2
                  (bind _returnvalue_3 (Game|SpawnActorfromClass "/Game/Blueprints/Characters/Tori/BattleMode/BP_Tori_Battler.BP_Tori_Battler_C" (Math|Transform|MakeTransform (Math|Vector|MakeVector (.X (Math|Vector|BreakVector (Transformation|GetWorldLocation (Variables|/Game/Blueprints/Game_Modes/BattleMode/BP_ColorPlatform.BP_ColorPlatform_C|GetDefaultSceneRoot (Utilities|Array|Get(acopy) _values _array_index))))) (- (.Y (Math|Vector|BreakVector (Transformation|GetWorldLocation (Variables|/Game/Blueprints/Game_Modes/BattleMode/BP_ColorPlatform.BP_ColorPlatform_C|GetDefaultSceneRoot (Utilities|Array|Get(acopy) _values _array_index))))) 25.0) (+ (.Z (Math|Vector|BreakVector (Transformation|GetWorldLocation (Variables|/Game/Blueprints/Game_Modes/BattleMode/BP_ColorPlatform.BP_ColorPlatform_C|GetDefaultSceneRoot (Utilities|Array|Get(acopy) _values _array_index))))) 1e+01))) "AlwaysSpawn" "MultiplyWithRoot" _self 0))
                  (LocalVariables|SetCreated%20Player _returnvalue_3))
                (:NewEnumerator3
                  (bind _returnvalue_4 (Game|SpawnActorfromClass "/Game/Blueprints/Characters/Jay/BattleMode/BP_Jay_Battler.BP_Jay_Battler_C" (Math|Transform|MakeTransform (Math|Vector|MakeVector (.X (Math|Vector|BreakVector (Transformation|GetWorldLocation (Variables|/Game/Blueprints/Game_Modes/BattleMode/BP_ColorPlatform.BP_ColorPlatform_C|GetDefaultSceneRoot (Utilities|Array|Get(acopy) _values _array_index))))) (- (.Y (Math|Vector|BreakVector (Transformation|GetWorldLocation (Variables|/Game/Blueprints/Game_Modes/BattleMode/BP_ColorPlatform.BP_ColorPlatform_C|GetDefaultSceneRoot (Utilities|Array|Get(acopy) _values _array_index))))) 25.0) (+ (.Z (Math|Vector|BreakVector (Transformation|GetWorldLocation (Variables|/Game/Blueprints/Game_Modes/BattleMode/BP_ColorPlatform.BP_ColorPlatform_C|GetDefaultSceneRoot (Utilities|Array|Get(acopy) _values _array_index))))) 1e+01))) "AlwaysSpawn" "MultiplyWithRoot" 0 0))
                  (LocalVariables|SetCreated%20Player _returnvalue_4))
                (:NewEnumerator4
                  (bind _returnvalue_5 (Game|SpawnActorfromClass "/Game/Blueprints/Characters/Lottie/BattleMode/BP_Lottie_Battler.BP_Lottie_Battler_C" (Math|Transform|MakeTransform (Math|Vector|MakeVector (.X (Math|Vector|BreakVector (Transformation|GetWorldLocation (Variables|/Game/Blueprints/Game_Modes/BattleMode/BP_ColorPlatform.BP_ColorPlatform_C|GetDefaultSceneRoot (Utilities|Array|Get(acopy) _values _array_index))))) (- (.Y (Math|Vector|BreakVector (Transformation|GetWorldLocation (Variables|/Game/Blueprints/Game_Modes/BattleMode/BP_ColorPlatform.BP_ColorPlatform_C|GetDefaultSceneRoot (Utilities|Array|Get(acopy) _values _array_index))))) 25.0) (+ (.Z (Math|Vector|BreakVector (Transformation|GetWorldLocation (Variables|/Game/Blueprints/Game_Modes/BattleMode/BP_ColorPlatform.BP_ColorPlatform_C|GetDefaultSceneRoot (Utilities|Array|Get(acopy) _values _array_index))))) 1e+01))) "AlwaysSpawn" "MultiplyWithRoot" 0 0))
                  (LocalVariables|SetCreated%20Player _returnvalue_5))
                (:NewEnumerator5
                  (bind _returnvalue_6 (Game|SpawnActorfromClass "/Game/Blueprints/Characters/Shio/BattleMode/BP_Shio_Battler.BP_Shio_Battler_C" (Math|Transform|MakeTransform (Math|Vector|MakeVector (.X (Math|Vector|BreakVector (Transformation|GetWorldLocation (Variables|/Game/Blueprints/Game_Modes/BattleMode/BP_ColorPlatform.BP_ColorPlatform_C|GetDefaultSceneRoot (Utilities|Array|Get(acopy) _values _array_index))))) (- (.Y (Math|Vector|BreakVector (Transformation|GetWorldLocation (Variables|/Game/Blueprints/Game_Modes/BattleMode/BP_ColorPlatform.BP_ColorPlatform_C|GetDefaultSceneRoot (Utilities|Array|Get(acopy) _values _array_index))))) 25.0) (+ (.Z (Math|Vector|BreakVector (Transformation|GetWorldLocation (Variables|/Game/Blueprints/Game_Modes/BattleMode/BP_ColorPlatform.BP_ColorPlatform_C|GetDefaultSceneRoot (Utilities|Array|Get(acopy) _values _array_index))))) 1e+01))) "AlwaysSpawn" "MultiplyWithRoot" 0 0))
                  (LocalVariables|SetCreated%20Player _returnvalue_6))))
            (:then_1
              ;[1 1 1] Set Platform Color
              (Sprite|SetSpriteColor (Variables|/Game/Blueprints/Game_Modes/BattleMode/BP_ColorPlatform.BP_ColorPlatform_C|GetPlatform%20Body (Utilities|Array|Get(acopy) _values _array_index)) (Default|GetCharacterColor (LocalVariables|GetCreated%20Player)))
              (Default|SetDirectionality (LocalVariables|GetCreated%20Player) "NewEnumerator0")
              (Variables|/Game/Blueprints/Game_Modes/BattleMode/BP_ColorPlatform.BP_ColorPlatform_C|SetLinked%20Battler (Utilities|Array|Get(acopy) _values _array_index) (LocalVariables|GetCreated%20Player)))))))))

(fn InputStateMachineTick
  (params (Direction :type ENUM_BattleInputDirections%20Enum :default "NewEnumerator0"))
  (switch Utilities|FlowControl|Switch|SwitchonENUM_BattleInputReceivers (Variables|Default|GetInput%20Mode)
    (:NewEnumerator0
      (switch Utilities|FlowControl|Switch|SwitchonENUM_BattleInputDirections Direction
        (:NewEnumerator0
          (CallFunction|MoveCellSelector Direction :!label _label))
        (:NewEnumerator1
          (goto _label))
        (:NewEnumerator2
          (goto _label))
        (:NewEnumerator3
          (goto _label))
        (:NewEnumerator4
          (bind _battler (CallFunction|GetCell (Variables|Default|GetSelected%20Cell) "PlayerPlatforms"))
          (if (Utilities|IsValidInterface _battler)
            (CallFunction|SetInputMode "NewEnumerator4")))))
    (:NewEnumerator4
      (Default|OnInputReceived (Variables|/Game/Blueprints/Game_Modes/GM_Battle.GM_Battle_C|GetWBP_BattleHUD (Variables|Default|GetBattle%20Game%20Mode)) Direction))
    (:NewEnumerator5
      (switch Utilities|FlowControl|Switch|SwitchonENUM_BattleInputDirections Direction
        (:NewEnumerator0
          (CallFunction|MoveCellSelector Direction :!label _label_2))
        (:NewEnumerator1
          (goto _label_2))
        (:NewEnumerator2
          (goto _label_2))
        (:NewEnumerator3
          (goto _label_2))
        (:NewEnumerator4
          (bind _active_event (CallFunction|GetActiveEvent))
          (Class|BattleEventContext|AddTargetCell _active_event (Variables|Default|GetSelected%20Cell) (.CurrentPlatformSelectMode (Utilities|Struct|BreakSTRUCT_BattleInputMetadata (Variables|Default|GetInput%20Metadata))))
          (if (== (Class|BattleEventContext|GetTargetCellCount _active_event) (Class|BattleActionBase|GetNumTargets (Variables|/Script/SummersEnd.BattleEventContext|Getm_action _active_event)))
            ;[1 1 1] Only call execute when max target cells have been reached
            (Class|BattleActionBase|CallExecute (Variables|/Script/SummersEnd.BattleEventContext|Getm_action _active_event) _active_event)))
        (:NewEnumerator5
          (CallFunction|SetInputMode "NewEnumerator4"))))
    (:NewEnumerator6
      (switch Utilities|FlowControl|Switch|SwitchonENUM_BattleInputDirections Direction
        (:NewEnumerator0
          (Default|OnInputReceived (Variables|/Game/Blueprints/Game_Modes/GM_Battle.GM_Battle_C|GetWBP_BattleHUD (Variables|Default|GetBattle%20Game%20Mode)) Direction :!label _label_3))
        (:NewEnumerator1
          (goto _label_3))
        (:NewEnumerator2
          (goto _label_3))
        (:NewEnumerator3
          (goto _label_3))
        (:NewEnumerator4
          (goto _label_3))
        (:NewEnumerator5
          (CallFunction|PopActiveContext)
          (bind _active_event_2 (CallFunction|GetActiveEvent))
          (Utilities|FlowControl|Sequence
            (:then_0
              (Utilities|IsValid _active_event_2
                (:Is%20Valid
                  (Utilities|FlowControl|Sequence
                    (:then_0
                      (Utilities|IsValid (Variables|/Script/SummersEnd.BattleEventContext|Getm_action _active_event_2)
                        (:Is%20Valid
                          (Class|BattleActionBase|CallUndo (Variables|/Script/SummersEnd.BattleEventContext|Getm_action _active_event_2) _active_event_2))))
                    (:then_1
                      (if (Utilities|Array|IsNotEmpty (Variables|/Script/SummersEnd.BattleEventContext|Getm_targetCells _active_event_2))
                        (bind _structout (Utilities|Struct|SetmembersinSTRUCT_BattleInputMetadata (Variables|Default|GetInput%20Metadata)))
                        (|SetBy-RefVar (.CurrentPlatformSelectMode (Utilities|Struct|BreakSTRUCT_BattleInputMetadata _structout)) (Variables|/Script/SummersEnd.SBattleGridCellData|Getm_type (Utilities|Array|Get(acopy) (Variables|/Script/SummersEnd.BattleEventContext|Getm_targetCells _active_event_2) (Utilities|Array|LastIndex (Variables|/Script/SummersEnd.BattleEventContext|Getm_targetCells _active_event_2)))))))))
                (:Is%20Not%20Valid
                  (Development|PrintString "Input State Machine Tick::Sub-action select cancel failed to get  context" true true "(R=1.000000,G=0.050508,B=0.000000,A=1.000000)" 1e+01 "ERROR"))))
            (:then_1
              (Class|BattleEventContext|PopTargetCells _active_event_2 1)
              ;[1 1 1] Can be customized for different effects by whatever condition
              (CallFunction|SetInputMode "NewEnumerator5"))))))))

(fn MoveCellSelector
  (params (Direction :type ENUM_BattleInputDirections%20Enum :default "NewEnumerator0"))
  (bind _selected_cell (Variables|Default|GetSelected%20Cell))
  (bind (_x _y) (Utilities|Struct|BreakIntPoint _selected_cell))
  (Utilities|FlowControl|Sequence
    (:then_0
      (switch Utilities|FlowControl|Switch|SwitchonENUM_BattleInputDirections Direction
        (:NewEnumerator0
          (LocalVariables|SetTarget%20Cell (Utilities|Struct|MakeIntPoint _x (- _y 1))))
        (:NewEnumerator1
          (LocalVariables|SetTarget%20Cell (Utilities|Struct|MakeIntPoint _x (+ _y 1))))
        (:NewEnumerator2
          (LocalVariables|SetTarget%20Cell (Utilities|Struct|MakeIntPoint (- _x 1) _y)))
        (:NewEnumerator3
          (LocalVariables|SetTarget%20Cell (Utilities|Struct|MakeIntPoint (+ _x 1) _y)))))
    (:then_1
      (CallFunction|HoverbyGridCell (LocalVariables|GetTarget%20Cell) (Variables|Default|GetSelected%20Cell)))))

(fn HoverbyGridCell
  (params (Target%20Cell :type Int%20Point%20Structure) (Source%20Cell :type Int%20Point%20Structure))
  (Utilities|FlowControl|Sequence
    (:then_0
      (bind _structout (Utilities|Struct|SetmembersinSTRUCT_BattleInputMetadata (Variables|Default|GetInput%20Metadata)))
      (Utilities|FlowControl|Sequence
        (:then_0
          (switch Utilities|FlowControl|Switch|SwitchonEBattlePlatformCollectionType (.LastPlatformSelectMode (Utilities|Struct|BreakSTRUCT_BattleInputMetadata _structout))
            (:PlayerPlatforms
              (CallFunction|SetHoverStatebyIndex false Source%20Cell (Variables|Default|GetPlayer%20Platforms)))
            (:EnemyPlatforms
              (CallFunction|SetHoverStatebyIndex false Target%20Cell (Variables|Default|GetEnemy%20Platforms)))
            (:AllPlatforms
              (CallFunction|SetHoverStatebyIndex false Target%20Cell (Variables|Default|GetAll%20Platforms)))))
        (:then_1
          (Variables|Default|SetSelected%20Cell Target%20Cell)
          (|SetBy-RefVar (.LastPlatformSelectMode (Utilities|Struct|BreakSTRUCT_BattleInputMetadata _structout)) (.CurrentPlatformSelectMode (Utilities|Struct|BreakSTRUCT_BattleInputMetadata _structout))))))
    (:then_2
      (switch Utilities|FlowControl|Switch|SwitchonEBattlePlatformCollectionType (.CurrentPlatformSelectMode (Utilities|Struct|BreakSTRUCT_BattleInputMetadata (Variables|Default|GetInput%20Metadata)))
        (:PlayerPlatforms
          (bind _platform (CallFunction|SetHoverStatebyIndex true Target%20Cell (Variables|Default|GetPlayer%20Platforms)))
          (return _platform))
        (:EnemyPlatforms
          (bind _platform_2 (CallFunction|SetHoverStatebyIndex true Target%20Cell (Variables|Default|GetEnemy%20Platforms)))
          (return _platform_2))
        (:AllPlatforms
          (bind _platform_3 (CallFunction|SetHoverStatebyIndex true Target%20Cell (Variables|Default|GetAll%20Platforms)))
          (return _platform_3))))))

(fn SetHoverStatebyIndex
  (params (Hovered :type Boolean%20%28by%20ref%29) (Cell :type Int%20Point%20Structure%20%28by%20ref%29) (Cell%20Collection :type STRUCT%20Battle%20Grid%20Cell%20Collection%20Structure%20%28by%20ref%29))
  (bind _gridcells (Utilities|Struct|BreakSTRUCT_BattleGridCellCollection Cell%20Collection))
  (bind (_value _returnvalue) (Utilities|Map|Find _gridcells Cell))
  (if _returnvalue
    (Default|OnHover _value Hovered)
    (return _value)
    (else
      (Development|PrintString "Set Hover State By Cell:: couldnt find cell to set state on")
      (return 0))))

(fn SetInputMode
  (params (Input%20Mode :type ENUM_BattleInputReceivers%20Enum :default "NewEnumerator0"))
  (if (Utilities|Enum|NotEqual(Enum) Input%20Mode (Variables|Default|GetInput%20Mode))
    (Utilities|FlowControl|Sequence
      (:then_0
        ;[1 1 1] The mode we're in
        (switch Utilities|FlowControl|Switch|SwitchonENUM_BattleInputReceivers (Variables|Default|GetInput%20Mode)
          (:NewEnumerator0
            ;[1 1 1] The mode we're going to
            (switch Utilities|FlowControl|Switch|SwitchonENUM_BattleInputReceivers Input%20Mode
              (:NewEnumerator4
                (Utilities|FlowControl|Sequence
                  (:then_0
                    (bind _active_event (CallFunction|GetActiveEvent))
                    (Class|BattleEventContext|SetSourceCell _active_event (Variables|Default|GetSelected%20Cell) (.CurrentPlatformSelectMode (Utilities|Struct|BreakSTRUCT_BattleInputMetadata (Variables|Default|GetInput%20Metadata)))))
                  (:then_1
                    (Default|ShowActionMenu (Variables|/Game/Blueprints/Game_Modes/GM_Battle.GM_Battle_C|GetWBP_BattleHUD (Variables|Default|GetBattle%20Game%20Mode)) true))))))
          (:NewEnumerator4
            (switch Utilities|FlowControl|Switch|SwitchonENUM_BattleInputReceivers Input%20Mode
              (:NewEnumerator0
                (CallFunction|ResetActiveEvent)
                (Default|ShowActionMenu (Variables|/Game/Blueprints/Game_Modes/GM_Battle.GM_Battle_C|GetWBP_BattleHUD (Variables|Default|GetBattle%20Game%20Mode)) false))
              (:NewEnumerator5
                (Default|ShowActionMenu (Variables|/Game/Blueprints/Game_Modes/GM_Battle.GM_Battle_C|GetWBP_BattleHUD (Variables|Default|GetBattle%20Game%20Mode)) false))))
          (:NewEnumerator5
            (switch Utilities|FlowControl|Switch|SwitchonENUM_BattleInputReceivers Input%20Mode
              (:NewEnumerator4
                (Default|ShowActionMenu (Variables|/Game/Blueprints/Game_Modes/GM_Battle.GM_Battle_C|GetWBP_BattleHUD (Variables|Default|GetBattle%20Game%20Mode)) true))
              (:NewEnumerator6
                (bind _active_event_2 (CallFunction|GetActiveEvent))
                (bind _returnvalue (Class|BattleFunctionLibraryFactory|CreateUBattleEventContext _active_event_2))
                (Class|BattleEventContext|SetChildContext _active_event_2 _returnvalue)
                (Class|BattleEventContext|SetParentContext _returnvalue _active_event_2)
                (Default|ShowActionMenu (Variables|/Game/Blueprints/Game_Modes/GM_Battle.GM_Battle_C|GetWBP_BattleHUD (Variables|Default|GetBattle%20Game%20Mode)) true))))
          (:NewEnumerator6
            (switch Utilities|FlowControl|Switch|SwitchonENUM_BattleInputReceivers Input%20Mode
              (:NewEnumerator5
                (Default|ShowActionMenu (Variables|/Game/Blueprints/Game_Modes/GM_Battle.GM_Battle_C|GetWBP_BattleHUD (Variables|Default|GetBattle%20Game%20Mode)) false))))))
      (:then_1
        (Variables|Default|SetInput%20Mode Input%20Mode)))))

(fn GetCell
  (params (Cell :type Int%20Point%20Structure) (Platform%20Type :type EBattlePlatformCollectionType%20Enum :default "PlayerPlatforms"))
  (bind _enemy_platforms (Variables|Default|GetEnemy%20Platforms))
  (bind _player_platforms (Variables|Default|GetPlayer%20Platforms))
  (bind _all_platforms (Variables|Default|GetAll%20Platforms))
  (bind _gridcells (Utilities|Struct|BreakSTRUCT_BattleGridCellCollection _player_platforms))
  (bind _gridcells_2 (Utilities|Struct|BreakSTRUCT_BattleGridCellCollection _enemy_platforms))
  (bind _gridcells_3 (Utilities|Struct|BreakSTRUCT_BattleGridCellCollection _all_platforms))
  (bind (_value _returnvalue) (Utilities|Map|Find _gridcells_3 Cell))
  (bind (_value_2 _returnvalue_2) (Utilities|Map|Find _gridcells Cell))
  (bind (_value_3 _returnvalue_3) (Utilities|Map|Find _gridcells_2 Cell))
  (switch Utilities|FlowControl|Switch|SwitchonEBattlePlatformCollectionType Platform%20Type
    (:PlayerPlatforms
      (if _returnvalue_2
        (return (Variables|/Game/Blueprints/Game_Modes/BattleMode/BP_ColorPlatform.BP_ColorPlatform_C|GetLinked%20Battler _value_2) _value_2)
        (else
          (return 0 0))))
    (:EnemyPlatforms
      (if _returnvalue_3
        (return (Variables|/Game/Blueprints/Game_Modes/BattleMode/BP_ColorPlatform.BP_ColorPlatform_C|GetLinked%20Battler _value_3) _value_3)
        (else
          (return 0 0))))
    (:AllPlatforms
      (if _returnvalue
        (return (Variables|/Game/Blueprints/Game_Modes/BattleMode/BP_ColorPlatform.BP_ColorPlatform_C|GetLinked%20Battler _value) _value)
        (else
          (return 0 0))))))

(fn ResetActiveEvent
  (bind _active_event (CallFunction|GetActiveEvent))
  (Class|BattleEventContext|Reset _active_event))

(fn GetActiveEvent
  (bind _event_queue (Variables|Default|GetEvent%20Queue))
  (bind _returnvalue (Utilities|Array|LastIndex _event_queue))
  (bind _output (Utilities|Array|Get(acopy) _event_queue _returnvalue))
  (bind _returnvalue_2 (Class|BattleEventContext|GetChildContext _output))
  (if (Utilities|IsValid _returnvalue_2)
    (bind _output_get (LocalVariables|SetChild%20Context%20Ref _returnvalue_2))
    (while (Utilities|IsValid (Class|BattleEventContext|GetChildContext (LocalVariables|GetChild%20Context%20Ref)))
      (LocalVariables|SetChild%20Context%20Ref (Class|BattleEventContext|GetChildContext (LocalVariables|GetChild%20Context%20Ref))))
    (return _output_get)
    (else
      (return _output))))

(fn SwapObjectsatCells
  (params (Cell%20A :type S%20Battle%20Grid%20Cell%20Data%20Object%20Reference) (Cell%20B :type S%20Battle%20Grid%20Cell%20Data%20Object%20Reference))
  (bind _color_platform (CallFunction|GetCell (Variables|/Script/SummersEnd.SBattleGridCellData|Getm_cell Cell%20A) (Variables|/Script/SummersEnd.SBattleGridCellData|Getm_type Cell%20A)))
  (if (Utilities|IsValid _color_platform)
    (bind (_battler _color_platform_2) (CallFunction|GetCell (Variables|/Script/SummersEnd.SBattleGridCellData|Getm_cell Cell%20B) (Variables|/Script/SummersEnd.SBattleGridCellData|Getm_type Cell%20B)))
    (if (Utilities|IsValid _color_platform_2)
      (bind _previous_battler (Default|SetBattler _color_platform _battler))
      (Default|SetBattler _color_platform_2 _previous_battler))))

(fn SetActiononActiveEvent
  (params (Action :type Battle%20Action%20Base%20Object%20Reference))
  (EventDispatchers|UnbindallEventsfromOnBattleExecute Action)
  (bind _active_event (CallFunction|GetActiveEvent))
  (Class|BattleEventContext|SetAction _active_event Action)
  (Utilities|IsValid Action
    (:Is%20Valid
      (CallFunction|BindtoBattleActionEvent Action))))

(fn PopActiveContext
  (bind _active_event (CallFunction|GetActiveEvent))
  (if (Utilities|IsValid (Class|BattleEventContext|GetParentContext _active_event))
    (Class|BattleEventContext|SetChildContext (Class|BattleEventContext|GetParentContext _active_event))))