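; A selectable colored platform for battle mode that holds one linked battler.
; Setting a battler tints the body sprite with that battler's color and moves it to the platform, or resets to white if invalid, returning the previously linked battler.
; Hovering toggles the selection border between the selected color and black and forwards the hover to the linked battler through its interface.
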(event EventBeginPlay)

(event Collision|EventActorBeginOverlap
  (params (OtherActor :type Actor%20Object%20Reference)))

(event EventTick
  (params (DeltaSeconds :type Float%20%28single-precision%29)))

(event EventOnHover
  (params (Hovered :type Boolean))
  (bind _linked_battler (Variables|Default|GetLinked%20Battler))
  (Utilities|FlowControl|Sequence
    (:then_0
      (CallFunction|SetSelected Hovered))
    (:then_1
      (if (Utilities|IsValidInterface _linked_battler)
        (Default|OnHover _linked_battler Hovered)))))

(fn ConstructionScript)

(fn SetSelected
  (params (Selected :type Boolean))
  (bind _selection_border (Variables|Default|GetSelection%20Border))
  (Utilities|FlowControl|Sequence
    (:then_0
      (Variables|Default|SetIs%20Selected Selected))
    (:then_1
      (if Selected
        (Sprite|SetSpriteColor _selection_border (Variables|Default|GetSelected%20Color))
        (else
          (Sprite|SetSpriteColor _selection_border "(R=0.000000,G=0.000000,B=0.000000,A=1.000000)"))))))

(fn GetIsSelected
  (return (Variables|Default|GetIs%20Selected)))

(fn SetBattler
  (params (Battler%20To%20Set :type BPI%20Battler%20Interface))
  (bind _platform_body (Variables|Default|GetPlatform%20Body))
  (Utilities|FlowControl|Sequence
    (:then_0
      (if (Utilities|IsValidInterface Battler%20To%20Set)
        (bind _color (Default|GetColor Battler%20To%20Set))
        (Sprite|SetSpriteColor _platform_body _color)
        (Default|UpdateBattlerPosition Battler%20To%20Set (Transformation|GetWorldLocation (Variables|Default|GetDefaultSceneRoot)))
        (else
          (Sprite|SetSpriteColor _platform_body "(R=1.000000,G=1.000000,B=1.000000,A=1.000000)"))))
    (:then_1
      (bind _output_get (LocalVariables|SetPrev%20Battler (Variables|Default|GetLinked%20Battler)))
      (Variables|Default|SetLinked%20Battler Battler%20To%20Set)
      (return _output_get))))