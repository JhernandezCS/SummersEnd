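; GM_MainGame is the main game mode, which creates the main HUD at BeginPlay and tracks the active level sequence.
; SetActiveSequence stores a new sequence unless the current one is still playing, in which case it prints a warning.
; It binds each stored sequence's pause event to resume playback immediately unless BPCCutsceneManager reports dialogue in progress.
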(event Custom|Bind%20To%20Active%20Sequence%20Pause
  (bind _active_sequence (Variables|Default|GetActive%20Sequence))
  (Utilities|IsValid _active_sequence
    (:Is%20Valid
      (EventDispatchers|BindEventtoOnPause _active_sequence (delegate Custom|Pause%20Active%20Sequence)))))

(event Custom|Pause%20Active%20Sequence
  (bind _active_sequence (Variables|Default|GetActive%20Sequence))
  (Utilities|IsValid _active_sequence
    (:Is%20Valid
      (if (not (Default|IsDialogueinProgress (Variables|Default|GetBPC_CutsceneManager)))
        (Sequencer|Player|Play _active_sequence :!class /Script/MovieScene.MovieSceneSequencePlayer)))))

(event EventBeginPlay
  (CallFunction|InitalizeHUD))

(event EventTick
  (params (DeltaSeconds :type Float%20%28single-precision%29)))

(fn ConstructionScript)

(fn InitalizeHUD
  (bind _returnvalue (UserInterface|CreateWidget "/Game/Widgets/WBP_MainHUD.WBP_MainHUD_C" (Game|GetPlayerController 0)))
  (UserInterface|Viewport|AddtoViewport _returnvalue 0)
  (Variables|Default|SetWBP_MainHUD _returnvalue))

(fn SetActiveSequence
  (params (Seq%20to%20Set :type Level%20Sequence%20Player%20Object%20Reference))
  (Utilities|IsValid (Variables|Default|GetActive%20Sequence)
    (:Is%20Valid
      (if (Audio|Components|Audio|IsPlaying (Variables|Default|GetActive%20Sequence))
        (Development|PrintString "GM_MainGame::SetActiveSequence already had a playing sequence")
        (else
          (Variables|Default|SetActive%20Sequence Seq%20to%20Set :!label _label)
          (CallFunction|BindtoActiveSequencePause))))
    (:Is%20Not%20Valid
      (goto _label))))

(fn GetActiveSequence
  (return (Variables|Default|GetActive%20Sequence)))