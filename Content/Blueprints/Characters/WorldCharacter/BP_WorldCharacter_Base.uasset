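; Base character Blueprint for world characters, holding shared movement and knockout state.
; It exposes getters and setters for running, knocked-out and force-stop-running flags, without acting on them here.
; The MoveToTargetAndHide event moves the capsule component to a target point over a set duration, then hides the actor in game.
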(event Custom|MoveToTargetAndHide
  (Components|MoveComponentTo (Variables|Default|GetCapsuleComponent) (Variables|Default|GetMoveToTargetPoint) "0, 0, 0" false false (Variables|Default|GetMoveToTargetDuration) false)
  (Rendering|SetActorHiddenInGame true))

(event EventBeginPlay)

(event Collision|EventActorBeginOverlap
  (params (OtherActor :type Actor%20Object%20Reference)))

(event EventTick
  (params (DeltaSeconds :type Float%20%28single-precision%29)))

(fn ConstructionScript)

(fn GetIsRunning
  (return (Variables|Default|GetIs%20Running)))

(fn SetIsRunning
  (params (Is%20Running :type Boolean))
  (Variables|Default|SetIs%20Running Is%20Running))

(fn SetIsKnockedOut
  (params (Knocked%20Out :type Boolean))
  (Variables|Default|SetIs%20Knocked%20Out Knocked%20Out))

(fn GetIsKnockedOut
  (return (Variables|Default|GetIs%20Knocked%20Out)))

(fn SetForceStopRunning
  (params (Force%20Stop :type Boolean))
  (Variables|Default|SetForce%20Stop%20Running Force%20Stop))

(fn GetForceStopRunning
  (return (Variables|Default|GetForce%20Stop%20Running)))