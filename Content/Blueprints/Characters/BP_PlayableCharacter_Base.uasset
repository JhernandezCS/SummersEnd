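; Base Blueprint for playable characters, handling movement input and the facing direction used by animation.
; BeginPlay caches the GM_MainGame game mode, printing an error if the cast fails.
; IA_Move moves the character along world X and Y and stores the input, with Y inverted, as Directionality.
; SetDirectionality sets that vector from a four-way direction; Left yields (-1, 1), unlike the other purely axial values.
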(event Input|EnhancedActionEvents|EnhancedInputActionIA_Move
  (params (ActionValue :type Vector%202D%20Structure) (ElapsedSeconds :type Float%20%28double-precision%29) (TriggeredSeconds :type Float%20%28double-precision%29) (InputAction :type Input%20Action%20Object%20Reference :default "/Game/Blueprints/Input/Actions/IA_Move.IA_Move"))
  (bind (_x _y) (Math|Vector2D|BreakVector2D ActionValue))
  (Utilities|FlowControl|Sequence
    (:then_0
      ;[1 1 1] Determines animation movement
      (Variables|Default|SetDirectionality (Math|Vector2D|MakeVector2D _x (* _y -1.0))))
    (:then_1
      (Pawn|Input|AddMovementInput "1.000000,0.000000,0.000000" _x false)
      (Pawn|Input|AddMovementInput "0.000000,1.000000,0.000000" _y false))))

(event EventBeginPlay
  (bind _asgm_main_game (Utilities|Casting|CastToGM_MainGame (Game|GetGameMode))
    (:then
      (Variables|Default|SetGM_MainGame _asgm_main_game))
    (:CastFailed
      (Development|PrintString "BP_PlayableCharacter::BeingPlay failed to cast game mode to GM_MainGame"))))

(event Collision|EventActorBeginOverlap
  (params (OtherActor :type Actor%20Object%20Reference)))

(event EventTick
  (params (DeltaSeconds :type Float%20%28single-precision%29)))

(fn ConstructionScript
  (|CallParentFunction))

(fn SetDirectionality
  (params (Direction :type ENUM_AnimationDirections%20Enum :default "NewEnumerator0"))
  (switch Utilities|FlowControl|Switch|SwitchonENUM_AnimationDirections Direction
    (:NewEnumerator0
      (Variables|Default|SetDirectionality "(X=0.000000,Y=1.000000)"))
    (:NewEnumerator1
      (Variables|Default|SetDirectionality "(X=0.000000,Y=-1.000000)"))
    (:NewEnumerator2
      (Variables|Default|SetDirectionality "(X=1.000000,Y=0.000000)"))
    (:NewEnumerator3
      (Variables|Default|SetDirectionality "(X=-1.000000,Y=1.000000)"))))