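; BP_Tori_Battler is Tori's battle-mode character Blueprint, adding a reaction to being hovered.
; OnHover switches the directionality between two enum values according to the hover state, then passes that state to SetIsRunning, so Tori runs while hovered.
; BeginPlay, overlap and Tick are disabled stubs, and the construction script only calls its parent.
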(event EventBeginPlay
  (|CallParentFunction) ; This node is disabled and will not be called.\nDrag off pins to build functionality.
)

(event Collision|EventActorBeginOverlap
  (params (OtherActor :type Actor%20Object%20Reference))
  (|CallParentFunction OtherActor) ; This node is disabled and will not be called.\nDrag off pins to build functionality.
)

(event EventTick
  (params (DeltaSeconds :type Float%20%28single-precision%29))
  (|CallParentFunction DeltaSeconds) ; This node is disabled and will not be called.\nDrag off pins to build functionality.
)

(event EventOnHover
  (params (Hovered :type Boolean))
  (Utilities|FlowControl|Sequence
    (:then_0
      (if Hovered
        (CallFunction|SetDirectionality "NewEnumerator1")
        (else
          (CallFunction|SetDirectionality "NewEnumerator0"))))
    (:then_1
      (CallFunction|SetIsRunning Hovered))))

(fn ConstructionScript
  (|CallParentFunction))